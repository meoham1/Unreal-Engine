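; BP_Pone is a test player pawn that moves and turns through Enhanced Input.
; On BeginPlay it casts its controller to PlayerController and adds the IMC mapping context.
; IA_Move drives movement along the control rotation's forward vector and yaw scaled by RotationRate.
; The scale values come from the action's triggered and elapsed seconds, not its input value.
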(event `EnhancedInput|/Game/ThirdPerson/Input/Actions/IA_Move`
  (params (ActionValue :type "Vector2D Structure") (ElapsedSeconds :type "Float (double-precision)") (TriggeredSeconds :type "Float (double-precision)") (InputAction :type "InputAction Object Reference" :default "/Game/ThirdPerson/Input/Actions/IA_Move.IA_Move"))
  (:`Triggered`
    (`self.AddMovementInput` (`KismetMathLibrary.GetForwardVector` (`self.GetControlRotation`)) TriggeredSeconds)
    (`self.AddControllerYawInput` (* ElapsedSeconds (`self.Rotation Rate`)))))

(event `self.ReceiveBeginPlay`
  (bind `_as플레이어_컨트롤러` (cast `PlayerController` (`self.GetController`)))
  (message `EnhancedInputSubsystemInterface.AddMappingContext` (pcsubsystem `EnhancedInputLocalPlayerSubsystem` `_as플레이어_컨트롤러`) "/Game/Test/2024-05-09/IMC.IMC" 0 (struct)))

(fn `UserConstructionScript`)