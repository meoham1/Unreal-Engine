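; Game mode for a test level that counts down remaining targets and opens a door when the last one is cleared.
; On BeginPlay it caches the first BP_DoorOpen actor in the world as the door reference.
; DecrementTarget lowers the target count, or, when only one remains, opens the door and hides every top-level BP_Interface widget.
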(event `self.ReceiveBeginPlay`
  (bind _outactors (`GameplayStatics.GetAllActorsOfClass` "/Game/Test/2024-05-31/1/BP_DoorOpen.BP_DoorOpen_C"))
  (set `self.DoorReference` (`|GetArrayItem` _outactors)))

(event `DecrementTarget`
  (bind _targetnum (`self.TargetNum`))
  (if (== _targetnum 1)
    (`/Game/Test/2024-05-31/1/BP_DoorOpen.OpenDoor` (`self.DoorReference`))
    (bind _foundwidgets (`WidgetBlueprintLibrary.GetAllWidgetsOfClass` "/Game/Test/2024-05-31/1/BP_Interface.BP_Interface_C"))
    (for _array_element _foundwidgets
      (bind _asbp_interface (cast `/Game/Test/2024-05-31/1/BP_Interface` _array_element))
      (`/Game/Test/2024-05-31/1/BP_Interface.HideWidget` _asbp_interface))
    (else
      (set `self.TargetNum` (- _targetnum 1)))))

(fn `UserConstructionScript`)