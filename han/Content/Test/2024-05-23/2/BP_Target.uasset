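; Shooting target that stands up or lies down, driven by two trigger actors that react to the third-person character.
; Entering ReadyTrigger sets the status to Up and leaving sets Ready; entering UpTrigger calls EventStandUp, then sets Ready.
; EventStandUp and Down act only from Ready and Up respectively, snapping TargetBoard's pitch and updating the status.
; Down has no caller here, and the TimeLine_Up timeline is unconnected.
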(event `self.readyTrigger.OnActorEndOverlap`
  (params (OverlappedActor :type "Actor Object Reference") (OtherActor :type "Actor Object Reference"))
  (cast `/Game/ThirdPerson/Blueprints/BP_ThirdPersonCharacter` OtherActor)
  (set `self.CurrentStatus` "NewEnumerator0"))

(event `self.upTrigger.OnActorBeginOverlap`
  (params (OverlappedActor :type "Actor Object Reference") (OtherActor :type "Actor Object Reference"))
  (cast `/Game/ThirdPerson/Blueprints/BP_ThirdPersonCharacter` OtherActor)
  (`KismetSystemLibrary.PrintString` "target up")
  (`self.EventStandUp`)
  (set `self.CurrentStatus` "NewEnumerator0"))

(event `self.readyTrigger.OnActorBeginOverlap`
  (params (OverlappedActor :type "Actor Object Reference") (OtherActor :type "Actor Object Reference"))
  (cast `/Game/ThirdPerson/Blueprints/BP_ThirdPersonCharacter` OtherActor)
  (`KismetSystemLibrary.PrintString` "ready to shot")
  (set `self.CurrentStatus` "NewEnumerator1"))

(event `Event Down`
  (switch `/Game/Test/2024-05-23/2/enum_TargetState` (`self.CurrentStatus`)
    (:`NewEnumerator1`
      (`SceneComponent.K2_SetRelativeRotation` (`self.targetBoard`) (`KismetMathLibrary.MakeRotator` 0.0 90.0) false false)
      (set `self.CurrentStatus` "NewEnumerator2"))))

(event `EventStandUp`
  (switch `/Game/Test/2024-05-23/2/enum_TargetState` (`self.CurrentStatus`)
    (:`NewEnumerator0`
      (`SceneComponent.K2_SetRelativeRotation` (`self.targetBoard`) (`KismetMathLibrary.MakeRotator` 0.0) false false)
      (set `self.CurrentStatus` "NewEnumerator1"))))

(fn `UserConstructionScript`)