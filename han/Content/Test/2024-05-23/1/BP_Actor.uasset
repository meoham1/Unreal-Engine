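; Test door actor that swings open on a yaw timeline when a BP_Cone actor enters its switch trigger.
; A separate lock trigger sets DoorLock when a cone overlaps it, and the open event plays the timeline only if that flag is true, otherwise printing "locked".
; A close event reverses the timeline, but nothing in this graph calls it.
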(event `self.doorLockTrg.OnActorBeginOverlap`
  (params (OverlappedActor :type "Actor Object Reference") (OtherActor :type "Actor Object Reference"))
  (cast `/Game/Test/2024-05-23/1/BP_Cone` OtherActor)
  (set `self.DoorLock` true)
  (`KismetSystemLibrary.PrintString` "locked"))

(event `EventOpenDoor`
  (if (`self.DoorLock`)
    (bind (_direction _doorrot) (`Timeline|타임라인` :!via `PlayFromStart` :!label _label)
      (:`Update`
        (`SceneComponent.K2_SetRelativeRotation` (`self.Door`) (`KismetMathLibrary.MakeRotator` 0.0 0.0 _doorrot) false false)))
    (else
      (`KismetSystemLibrary.PrintString` "locked"))))

(event `EventCloseDoor`
  (goto _label :!via `ReverseFromEnd`))

(event `self.ReceiveActorBeginOverlap`
  (params (OtherActor :type "Actor Object Reference")))

(event `self.doorSwitchTrg.OnActorBeginOverlap`
  (params (OverlappedActor :type "Actor Object Reference") (OtherActor :type "Actor Object Reference"))
  (cast `/Game/Test/2024-05-23/1/BP_Cone` OtherActor)
  (`KismetSystemLibrary.PrintString` "Hello")
  (`self.EventOpenDoor`))

(fn `UserConstructionScript`)